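; BP_Dodecagon builds a twelve-node figure out of spawned sphere and line actors on BeginPlay.
; It places a BP_Sphere at each NodePositions entry, with position and size multiplied by Scale.
; From each node it spawns BP_Line actors aimed at nodes at odd index offsets, subtracting 12 to wrap past the last.
; Each line's scale comes from its LineLengths entry times Scale.
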(event EventBeginPlay
  (bind _nodepositions (Variables|Default|GetNodePositions))
  (bind _scale (Variables|Default|GetScale))
  (bind _scale_2 (Variables|Default|GetScale))
  ;[1 1 1] spawn the 12 node spheres
  (for _array_element _nodepositions
    (Game|SpawnActorfromClass "/Game/Geometry/BP_Sphere.BP_Sphere_C" (Math|Transform|MakeTransform (* _array_element _scale) "0, 0, 0" (Math|Conversions|ToVector(Float) _scale)) "Undefined" 0 0))
  ;[1 1 1] for each node, make 6 lines that point to other nodes
  (for (_array_element_2 _array_index) _nodepositions
    (for (_array_element_3 _array_index_2) (Variables|Default|GetLineLengths)
      ;[1 1 1] make sure that we're accessing a valid index, in case the number is greater than 11
      (if (> (+ _array_index (+ (* _array_index_2 2) 1)) (Class|KismetSystemLibrary|MakeLiteralInteger 11))
        (Game|SpawnActorfromClass "/Game/Geometry/BP_Line.BP_Line_C" (Math|Transform|MakeTransform (* _scale_2 _array_element_2) (Math|Rotator|FindLookatRotation _array_element_2 (Utilities|Array|Get(acopy) _nodepositions (- (+ _array_index (+ (* _array_index_2 2) 1)) 12))) (* _scale_2 _array_element_3)) "Undefined" 0 0)
        (else
          (Game|SpawnActorfromClass "/Game/Geometry/BP_Line.BP_Line_C" (Math|Transform|MakeTransform (* _scale_2 _array_element_2) (Math|Rotator|FindLookatRotation _array_element_2 (Utilities|Array|Get(acopy) _nodepositions (+ _array_index (+ (* _array_index_2 2) 1)))) (* _scale_2 _array_element_3)) "Undefined" 0 0))))))

(fn ConstructionScript)