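; BP_RandomSpawner is an actor that randomizes the appearance of a mesh and its floor on begin play and each Jump press.
; It enables input from player 0 so the actor itself receives the Jump action.
; Change picks a random mesh, material and yaw for the StaticMesh component, and a separately random material from the same array for the floor.
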(event EventBeginPlay
  (Input|EnableInput (Game|GetPlayerController 0))
  (CallFunction|Change))

(event EventTick
  (params (DeltaSeconds :type Float%20%28single-precision%29)))

(event Input|ActionEvents|InputActionJump
  (params (Key :type Key%20Structure :default "None"))
  (:Pressed
    (CallFunction|Change)))

(fn ConstructionScript)

(fn Change
  (Components|StaticMesh|SetStaticMesh (Variables|Default|GetStaticMesh) (.OutItem (Utilities|Array|Random (Variables|Default|GetMeshes))))
  (Rendering|Material|SetMaterial (Variables|Default|GetStaticMesh) 0 (.OutItem (Utilities|Array|Random (Variables|Default|GetMaterials))))
  (Transformation|SetRelativeRotation (Variables|Default|GetStaticMesh) (Math|Rotator|MakeRotator 0.0 0.0 (Math|Random|RandomFloatinRange 0.0 3.6e+02)) false false)
  (Rendering|Material|SetMaterial (Variables|Default|GetFloor_400x400_Centered) 0 (.OutItem (Utilities|Array|Random (Variables|Default|GetMaterials)))))